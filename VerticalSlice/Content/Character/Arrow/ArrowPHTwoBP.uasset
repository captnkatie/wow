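; Player bow arrow projectile that damages enemies or, when the bow is concussive, briefly stuns them instead.
; Damage scales linearly from X velocity sampled just after spawn, and each tick aligns pitch with velocity.
; Overlapping an Enemy mesh reports an AI damage event and briefly blocks further hits.
; Concussive hits zero the target's walk speed, then a delay restores it and clears the bow's concussive flag.
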(event Custom|DamageDelay
  (bind _possstunnedactor (Variables|Default|GetPossStunnedActor))
  (bind _bowactor (Variables|Default|GetBowActor))
  (bind _returnvalue (Actor|GetComponentbyClass _possstunnedactor "/Script/Engine.CharacterMovementComponent"))
  ;[1 1 1] Hit Enemy
  (Utilities|FlowControl|Delay 0.2)
  (Variables|Default|SetHitEnemy false)
  (if (Variables|Default|GetCanConcuss)
    (Utilities|FlowControl|Delay 1.3)
    (if (Utilities|IsValid _returnvalue)
      (Variables|/Script/Engine.CharacterMovementComponent|SetMaxWalkSpeed _returnvalue (Variables|Default|GetSpeedHolder))
      (if (Utilities|IsValid _bowactor)
        (Variables|/Game/Assets/Evelyn/Weapons/Bow/BowBP.BowBP_C|SetIsConcussive _bowactor false)))))

(event Custom|ArrowAngleTwo
  (bind _returnvalue (Transformation|GetActorRotation))
  (bind (_roll _pitch _yaw) (Math|Rotator|BreakRotator _returnvalue))
  ;[1 1 1] Adjust Arrow Angle
  (Transformation|SetActorRotation (Math|Rotator|MakeRotator _roll (.Pitch (Math|Rotator|BreakRotator (Math|Rotator|MakeRotfromX (Transformation|GetVelocity)))) _yaw)))

(event EventBeginPlay
  ;[1 1 1] Spawn Values
  (bind _asmy_vschar_cont (Utilities|Casting|CastToMyVSCharCont (Game|GetPlayerController 0)))
  (bind _asbow_bp (Utilities|Casting|CastToBowBP (Variables|/Game/Character/MyVSCharCont.MyVSCharCont_C|GetEWActor _asmy_vschar_cont)))
  (bind _output_get (Variables|Default|SetBowActor _asbow_bp))
  (if (Variables|/Game/Assets/Evelyn/Weapons/Bow/BowBP.BowBP_C|GetIsConcussive _output_get)
    (Variables|Default|SetCanConcuss true))
  (Utilities|FlowControl|Delay 0.05)
  (Variables|Default|SetArrowDamage (Math|Float|Round (+ (* (.X (Math|Vector|BreakVector (Variables|/Script/Engine.MovementComponent|GetVelocity (Variables|Default|GetProjectileMovement)))) 0.0016) 4.0426))))

(event Collision|EventActorBeginOverlap
  (params (OtherActor :type Actor%20Object%20Reference))
  (bind _returnvalue (Actor|GetComponentbyClass OtherActor "/Script/Engine.SkeletalMeshComponent"))
  (bind _self self)
  ;[1 1 1] Hit Enemy
  (Variables|Default|SetPossStunnedActor OtherActor)
  (if (not (Variables|Default|GetHitEnemy))
    (if (Utilities|IsValid _returnvalue)
      (switch Utilities|FlowControl|Switch|SwitchonECollisionChannel (Collision|GetCollisionObjectType _returnvalue)
        (:ECC_GameTraceChannel3
          (if (Variables|Default|GetCanConcuss)
            (Variables|Default|SetSpeedHolder (Class|MovementComponent|GetMaxSpeed (Actor|GetComponentbyClass (Variables|Default|GetPossStunnedActor) "/Script/Engine.CharacterMovementComponent")))
            (Variables|/Script/Engine.CharacterMovementComponent|SetMaxWalkSpeed (Actor|GetComponentbyClass (Variables|Default|GetPossStunnedActor) "/Script/Engine.CharacterMovementComponent") 0.0)
            (else
              (bind _returnvalue_2 (Game|Damage|ApplyDamage OtherActor (Math|Conversions|ToFloat(Integer) (Variables|Default|GetArrowDamage)) 0 0))))
          (Class|AISenseDamage|ReportDamageEvent OtherActor _self _returnvalue_2 (Transformation|GetActorLocation _self))
          (Variables|Default|SetHitEnemy true)
          (CallFunction|DamageDelay))))))

(event EventTick
  (params (DeltaSeconds :type Float%20%28single-precision%29))
  ;[1 1 1] Adjust Arrow Angle
  (CallFunction|ArrowAngleTwo)
  (if true
    _))

(fn ConstructionScript)