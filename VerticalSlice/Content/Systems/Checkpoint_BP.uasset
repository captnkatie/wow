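; Checkpoint actor that saves the player's location when its Trigger component is overlapped.
; Any overlap stores player 0's MyVSChar location, whatever actor entered, and prints a debug message.
; It then writes that location to PlayerLocS in a Save_BP save in slot "check", updating the existing save or creating one if none exists.
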(event OnComponentBeginOverlap(Trigger)
  (params (OverlappedComponent :type Primitive%20Component%20Object%20Reference) (OtherActor :type Actor%20Object%20Reference) (OtherComp :type Primitive%20Component%20Object%20Reference) (OtherBodyIndex :type Integer) (bFromSweep :type Boolean) (SweepResult :type Hit%20Result%20Structure%20%28by%20ref%29))
  (Utilities|FlowControl|Sequence
    (:then_0
      (bind _asmy_vschar (Utilities|Casting|CastToMyVSChar (Game|GetPlayerCharacter 0)))
      (Variables|Default|SetPlayerLocation (Transformation|GetActorLocation _asmy_vschar))
      (Development|PrintString "Checkpoint Reached"))
    (:then_1
      (bind _returnvalue (SaveGame|DoesSaveGameExist "check"))
      (if _returnvalue
        (bind _returnvalue_2 (SaveGame|LoadGamefromSlot "check"))
        (bind _assave_bp (Utilities|Casting|CastToSave_BP _returnvalue_2))
        (Variables|/Game/Systems/Save_BP.Save_BP_C|SetPlayerLoc_S _assave_bp (Variables|Default|GetPlayerLocation))
        (SaveGame|SaveGametoSlot _assave_bp "check")
        (else
          (bind _returnvalue_3 (SaveGame|CreateSaveGameObject "/Game/Systems/Save_BP.Save_BP_C"))
          (Variables|/Game/Systems/Save_BP.Save_BP_C|SetPlayerLoc_S _returnvalue_3 (Variables|Default|GetPlayerLocation))
          (SaveGame|SaveGametoSlot _returnvalue_3 "check"))))))

(event EventBeginPlay)

(event Collision|EventActorBeginOverlap
  (params (OtherActor :type Actor%20Object%20Reference)))

(event EventTick
  (params (DeltaSeconds :type Float%20%28single-precision%29)))

(fn ConstructionScript)