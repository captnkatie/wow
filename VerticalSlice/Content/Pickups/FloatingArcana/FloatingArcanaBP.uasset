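; Floating arcana pickup that restores a MyVSChar player's CurrentArcana and destroys itself when collected.
; An outer pull collision starts a timeline that lerps the pickup from its current location toward the player's live position, so it homes in.
; The inner pickup collision adds ArcanaAmount without clamping the result.
; Both overlaps act only while the player's arcana is below maximum, checked once at overlap.
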(event OnComponentBeginOverlap(FAPickupColl)
  (params (OverlappedComponent :type Primitive%20Component%20Object%20Reference) (OtherActor :type Actor%20Object%20Reference) (OtherComp :type Primitive%20Component%20Object%20Reference) (OtherBodyIndex :type Integer) (bFromSweep :type Boolean) (SweepResult :type Hit%20Result%20Structure%20%28by%20ref%29))
  (bind _asmy_vschar (Utilities|Casting|CastToMyVSChar OtherActor))
  (if (< (Variables|/Game/Character/MyVSChar.MyVSChar_C|GetCurrentArcana _asmy_vschar) (Variables|/Game/Character/MyVSChar.MyVSChar_C|GetMaxArcana _asmy_vschar))
    (Variables|/Game/Character/MyVSChar.MyVSChar_C|SetCurrentArcana _asmy_vschar (+ (Variables|/Game/Character/MyVSChar.MyVSChar_C|GetCurrentArcana _asmy_vschar) (Variables|Default|GetArcanaAmount)))
    (Actor|DestroyActor)))

(event OnComponentBeginOverlap(PullToPlayerCollision)
  (params (OverlappedComponent :type Primitive%20Component%20Object%20Reference) (OtherActor :type Actor%20Object%20Reference) (OtherComp :type Primitive%20Component%20Object%20Reference) (OtherBodyIndex :type Integer) (bFromSweep :type Boolean) (SweepResult :type Hit%20Result%20Structure%20%28by%20ref%29))
  ;[1 1 1] Pulls Arcana to Player on Overlap
  (bind _asmy_vschar (Utilities|Casting|CastToMyVSChar OtherActor))
  (if (< (Variables|/Game/Character/MyVSChar.MyVSChar_C|GetCurrentArcana _asmy_vschar) (Variables|/Game/Character/MyVSChar.MyVSChar_C|GetMaxArcana _asmy_vschar))
    (bind _pullcollision (Timeline|Timeline_0 Play)
      (:Update
        (Transformation|SetActorLocation (Math|Vector|Lerp(Vector) (Transformation|GetActorLocation) (Transformation|GetActorLocation _asmy_vschar) _pullcollision) false false)))))

(event EventBeginPlay)

(event Collision|EventActorBeginOverlap
  (params (OtherActor :type Actor%20Object%20Reference)))

(event EventTick
  (params (DeltaSeconds :type Float%20%28single-precision%29)))

(fn ConstructionScript)