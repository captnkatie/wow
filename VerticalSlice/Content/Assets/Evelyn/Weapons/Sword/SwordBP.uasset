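; Evelyn's sword weapon Blueprint, which damages skeletal-mesh actors of the Enemy object type on overlap.
; Normal hits apply sword damage, then block further hits for 0.3 seconds.
; In corrosive mode, a new target is only recorded, and repeat overlaps run a five-pass damage loop.
; That loop contains a Delay and is gated by a counter that is reset but never incremented here.
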(event Custom|DamageDelay
  (Utilities|FlowControl|Delay 0.3)
  (Variables|Default|SetHitEnemy false))

(event Collision|EventActorBeginOverlap
  (params (OtherActor :type Actor%20Object%20Reference))
  (bind _returnvalue (Actor|GetComponentbyClass OtherActor "/Script/Engine.SkeletalMeshComponent"))
  ;[1 1 1] Regular Damage
  (Variables|Default|SetMostRecentHit OtherActor)
  (if (not (Variables|Default|GetHitEnemy))
    (if (Utilities|IsValid _returnvalue)
      (switch Utilities|FlowControl|Switch|SwitchonECollisionChannel (Collision|GetCollisionObjectType _returnvalue)
        (:ECC_GameTraceChannel3
          (if (Variables|Default|GetIsCorrosive)
            (if (== (Variables|Default|GetMostRecentHit) (Variables|Default|GetRecentCorrosiveHit))
              (if (< (Variables|Default|GetCorrosiveCounter) 3)
                (for _index (range 0 4)
                  (Game|Damage|ApplyDamage (stale _output_get) (Math|Conversions|ToFloat(Integer) (Variables|Default|GetCorrosiveDamage)) 0 0)
                  (Utilities|FlowControl|Delay (Variables|Default|GetCorrosiveDelay))))
              (else
                (bind _output_get (Variables|Default|SetRecentCorrosiveHit (Variables|Default|GetMostRecentHit)))
                (Variables|Default|SetCorrosiveCounter 0)))
            (else
              (Game|Damage|ApplyDamage OtherActor (Math|Conversions|ToFloat(Integer) (Variables|Default|GetSwordDamage)) 0 0)
              (Variables|Default|SetHitEnemy true)
              (CallFunction|DamageDelay))))))))

(fn ConstructionScript)